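; Samsung washing machine actor in the Quiz folder that presents different parts of the appliance through animation and movement.
; The AnimacjaDrzwiPralka event switches on an animation index to show idle, control panel, drawer, door or back.
; Each part plays a skeletal animation and eases the mesh to a preset relative pose with MoveComponentTo, delayed for door and back.
; Idle resets the mesh instantly and loops, while the panel view settles into its own looping idle.
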(event Custom|AnimacjaDrzwiPralka
  (params (animationIndex :type Integer))
  (bind _skeletalmesh (Variables|Default|GetSkeletalMesh))
  (bind _skeletalmesh_2 (Variables|Default|GetSkeletalMesh))
  (switch int animationIndex
    (:1
      (Components|MoveComponentTo _skeletalmesh "0.000000,0.000000,0.000000" "0, 0, 0" false false 0.0 false)
      (Components|Animation|PlayAnimation _skeletalmesh "/Game/pralkasamsung_2/SK_Pralka_samsung_v7_Anim_Rig_pralka_Idle.SK_Pralka_samsung_v7_Anim_Rig_pralka_Idle" true))
    (:2
      (Components|Animation|PlayAnimation _skeletalmesh_2 "/Game/pralkasamsung_2/SK_Pralka_samsung_v7_Anim_Rig_pralka_Panel.SK_Pralka_samsung_v7_Anim_Rig_pralka_Panel" false)
      (Components|MoveComponentTo _skeletalmesh_2 "0.000000,40.000000,-30.000000" "0.000000,30.000000,10.000000" false false 1.0 false)
      (Components|Animation|PlayAnimation _skeletalmesh_2 "/Game/pralkasamsung_2/SK_Pralka_samsung_v7_Anim_Rig_pralka_Panel_Idle.SK_Pralka_samsung_v7_Anim_Rig_pralka_Panel_Idle" true))
    (:3
      (Components|Animation|PlayAnimation (Variables|Default|GetSkeletalMesh) "/Game/pralkasamsung_2/SK_Pralka_samsung_v7_Anim_Rig_pralka_Szuflada.SK_Pralka_samsung_v7_Anim_Rig_pralka_Szuflada" false)
      (Components|MoveComponentTo (Variables|Default|GetSkeletalMesh) "-10.000000,30.000000,-30.000000" "0.000000,-15.000000,8.000000" false false 1.0 false))
    (:4
      (Components|Animation|PlayAnimation (Variables|Default|GetSkeletalMesh) "/Game/pralkasamsung_2/SK_Pralka_samsung_v7_Anim_Rig_pralka_Drzwi.SK_Pralka_samsung_v7_Anim_Rig_pralka_Drzwi" false)
      (Utilities|FlowControl|Delay 1.0)
      (Components|MoveComponentTo (Variables|Default|GetSkeletalMesh) "10.000000,25.000000,-5.000000" "0.000000,30.000000,10.000000" false false 1.0 false))
    (:5
      (Components|Animation|PlayAnimation (Variables|Default|GetSkeletalMesh) "/Game/pralkasamsung_2/SK_Pralka_samsung_v7_Anim_Rig_pralka_Tyl.SK_Pralka_samsung_v7_Anim_Rig_pralka_Tyl" false)
      (Utilities|FlowControl|Delay 1.5)
      (Components|MoveComponentTo (Variables|Default|GetSkeletalMesh) "-15.000000,60.000000,-30.000000" "0.000000,185.000000,0.000000" false false 1.5 false))))

(event EventBeginPlay)

(event Collision|EventActorBeginOverlap
  (params (OtherActor :type Actor%20Object%20Reference)))

(event EventTick
  (params (DeltaSeconds :type Float%20%28single-precision%29)))

(fn ConstructionScript)